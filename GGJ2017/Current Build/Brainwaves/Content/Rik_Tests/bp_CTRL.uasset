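; Test controller that, once Space is pressed, fades the sky sphere's background shade to red and makes a red cube disappear.
; The construction script creates a dynamic material instance on SkySphere.
; Tick repeatedly lerps its Bg_Shade parameter from the current value toward red, giving a frame-rate-dependent ease-out.
; When the color is near the target, it hides the first Bp_redcube found and disables its collision.
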(event EventBeginPlay)

(event Collision|EventActorBeginOverlap
  (params (OtherActor :type Actor%20Object%20Reference)))

(event EventTick
  (params (DeltaSeconds :type Float%20%28single-precision%29))
  (bind _linearcolor (Utilities|Struct|MakeLinearColor 1.0 0.07 0.070142 1.0))
  (bind _skysphere_mat (Variables|Default|GetSkySphere_Mat))
  (if (Variables|Default|GetGOGOGO)
    (bind _returnvalue (Rendering|Material|GetVectorParameterValue _skysphere_mat "Bg_Shade" :!class /Script/Engine.MaterialInstanceDynamic))
    (Rendering|Material|SetVectorParameterValue _skysphere_mat "Bg_Shade" (Math|Color|Lerp(LinearColor) _returnvalue _linearcolor 0.1) :!class /Script/Engine.MaterialInstanceDynamic)
    (if (Math|Vector|Equal(Vector) (Math|Conversions|ToVector(LinearColor) _returnvalue) (Math|Conversions|ToVector(LinearColor) _linearcolor) 0.1)
      (bind _outactors (Actor|GetAllActorsOfClass "/Game/Rik_Tests/bp_redcube.bp_redcube_C"))
      (Collision|SetCollisionEnabled (Variables|/Game/Rik_Tests/bp_redcube.bp_redcube_C|GetCube (Utilities|Array|Get(acopy) _outactors)) "NoCollision")
      (Rendering|SetVisibility (Variables|/Game/Rik_Tests/bp_redcube.bp_redcube_C|GetCube (Utilities|Array|Get(acopy) _outactors)) false false))))

(event Input|KeyboardEvents|SpaceBar
  (params (Key :type Key%20Structure :default "AnyKey"))
  (:Pressed
    (Variables|Default|SetGOGOGO true)))

(fn ConstructionScript
  (bind _skysphere (Variables|Default|GetSkySphere))
  (bind _returnvalue (Rendering|Material|CreateDynamicMaterialInstance _skysphere 0 (Rendering|Material|GetMaterial _skysphere 0) :!class /Script/Engine.PrimitiveComponent))
  (Variables|Default|SetSkySphere_Mat _returnvalue))