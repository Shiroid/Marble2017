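; Test ping ball that triggers a material-driven ping effect when it hits something hard enough.
; On hit, impact force is the length of velocity times hit normal; it must exceed a threshold and, during an active ping, the last force.
; A timeline writes hit location, opacity and a force-scaled radius to the Mpc_Ping parameter collection.
; Tick prints the force value for debugging.
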(event Custom|DriveHitVFX
  (Rendering|Material|SetVectorParameterValue "/Game/Rik_Tests/Ping_Test/Mpc_Ping.Mpc_Ping" "HitLocation" (Math|Conversions|ToLinearColor(Vector) (Variables|Default|GetLastHitLocation)) :!class /Script/Engine.KismetMaterialLibrary)
  (bind (_direction _radius_blend _opacity) (Timeline|TL_Ping PlayFromStart)
    (:Update
      (Rendering|Material|SetScalarParameterValue "/Game/Rik_Tests/Ping_Test/Mpc_Ping.Mpc_Ping" "PingOpacity" _opacity :!class /Script/Engine.KismetMaterialLibrary)
      (Rendering|Material|SetScalarParameterValue "/Game/Rik_Tests/Ping_Test/Mpc_Ping.Mpc_Ping" "HitRadius" (Math|Float|Lerp 0.0 (+ (* (Variables|Default|GetLastHitForce) 1.0) 2e+01) _radius_blend) :!class /Script/Engine.KismetMaterialLibrary))
    (:Finished
      (Variables|Default|SetGotHit false))))

(event EventBeginPlay)

(event Collision|EventActorBeginOverlap
  (params (OtherActor :type Actor%20Object%20Reference)))

(event EventTick
  (params (DeltaSeconds :type Float%20%28single-precision%29))
  (Development|PrintString (Utilities|String|ToString(Float) (Math|Vector|VectorLength (* (Transformation|GetComponentVelocity (Variables|Default|GetSphere)) (stale Collision|EventHit HitNormal)))) true true "(R=0.000000,G=0.660000,B=1.000000,A=1.000000)" 0.0))

(event Collision|EventHit
  (params (MyComp :type Primitive%20Component%20Object%20Reference) (Other :type Actor%20Object%20Reference) (OtherComp :type Primitive%20Component%20Object%20Reference) (bSelfMoved :type Boolean) (HitLocation :type Vector) (HitNormal :type Vector) (NormalImpulse :type Vector :default "0, 0, 0") (Hit :type Hit%20Result%20Structure%20%28by%20ref%29))
  (bind _returnvalue (Transformation|GetComponentVelocity MyComp))
  (bind _returnvalue_2 (* _returnvalue HitNormal))
  (bind _returnvalue_3 (Math|Vector|VectorLength _returnvalue_2))
  (if (> _returnvalue_3 (Variables|Default|GetLastHitForce))
    (if (> _returnvalue_3 (Variables|Default|GetForceToPingReq)) :!label _label
      (Variables|Default|SetLastHitForce _returnvalue_3)
      (Variables|Default|SetLastHitLocation (.ImpactPoint (Collision|BreakHitResult Hit)))
      (Variables|Default|SetGotHit true)
      (CallFunction|DriveHitVFX))
    (elif (not (Variables|Default|GetGotHit))
      (goto _label))))

(fn ConstructionScript)