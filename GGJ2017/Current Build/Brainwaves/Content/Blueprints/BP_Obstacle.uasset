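; BP_Obstacle is an obstacle actor that runs an unfinished line-of-sight test involving the level camera.
; BeginPlay caches the first CameraActor found.
; Each Tick traces on Visibility from its root toward the negated camera X and Y, ignoring all BP_BallCharacter actors, with persistent debug lines.
; The hit result is unused, and the node that disables the Box's collision is unconnected.
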(event EventBeginPlay
  (bind _outactors (Actor|GetAllActorsOfClass "/Script/Engine.CameraActor"))
  (Variables|Default|SetCamera (Utilities|Array|Get(acopy) _outactors)))

(event Collision|EventActorBeginOverlap
  (params (OtherActor :type Actor%20Object%20Reference)))

(event EventTick
  (params (DeltaSeconds :type Float%20%28single-precision%29))
  (bind _camera (Variables|Default|GetCamera))
  (bind _returnvalue (Transformation|GetActorLocation _camera))
  (bind _returnvalue_2 (Math|Vector|NegateVector _returnvalue))
  (bind _outactors (Actor|GetAllActorsOfClass "/Game/Blueprints/BP_BallCharacter.BP_BallCharacter_C"))
  (bind _outhit (Collision|LineTraceByChannel (Transformation|GetWorldLocation (Variables|Default|GetDefaultSceneRoot)) (Math|Vector|MakeVector (.x _returnvalue_2) (.y _returnvalue_2) 0.0) "TraceTypeQuery1" false _outactors "Persistent")))

(fn ConstructionScript)