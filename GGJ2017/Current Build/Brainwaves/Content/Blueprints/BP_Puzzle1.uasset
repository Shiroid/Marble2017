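; BP_Puzzle1 is an unfinished puzzle actor that reads player input to reset and inspect its own rotation.
; Back snaps its rotation to zero, while the left and right bumpers print its current yaw and pitch for debugging.
; The right-stick axis events and the Player component's hit event are empty.
; Disconnected leftovers hint at speed-scaled stick rotation and a work-in-progress EffectPlane spawn on hit.
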(event OnComponentHit(Player)
  (params (HitComponent :type Primitive%20Component%20Object%20Reference) (OtherActor :type Actor%20Object%20Reference) (OtherComp :type Primitive%20Component%20Object%20Reference) (NormalImpulse :type Vector :default "0, 0, 0") (Hit :type Hit%20Result%20Structure%20%28by%20ref%29))
  ;[1 1 1] Spawn Effect WIP
)

(event Input|ActionEvents|InputActionRightBumper
  (params (Key :type Key%20Structure :default "AnyKey"))
  (:Pressed
    (Development|PrintString (Utilities|String|ToString(Float) (.pitch (Transformation|GetActorRotation))))))

(event Input|ActionEvents|InputActionLeftBumper
  (params (Key :type Key%20Structure :default "AnyKey"))
  (:Pressed
    (Development|PrintString (Utilities|String|ToString(Float) (.yaw (Transformation|GetActorRotation))))))

(event Input|ActionEvents|InputActionBack
  (params (Key :type Key%20Structure :default "AnyKey"))
  (:Pressed
    (Transformation|SetActorRotation "0, 0, 0")))

(event Input|AxisEvents|InputAxisRightX
  (params (AxisValue :type Float%20%28single-precision%29)))

(event Input|AxisEvents|InputAxisRightY
  (params (AxisValue :type Float%20%28single-precision%29)))

(fn ConstructionScript)